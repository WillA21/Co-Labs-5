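; BP_Bubble is a bubble actor that launches the first-person player straight up on contact.
; It caches the player character on BeginPlay, and the player's first overlap with the Box activates its InterpToMovement component once.
; Capsule overlap applies the vertical launch, then hides the Sphere and disables its collision.
; It also sets a timer for a "Wait" function, which is not defined in this graph.
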(event OnComponentBeginOverlap(Capsule)
  (params (OverlappedComponent :type Primitive%20Component%20Object%20Reference) (OtherActor :type Actor%20Object%20Reference) (OtherComp :type Primitive%20Component%20Object%20Reference) (OtherBodyIndex :type Integer) (bFromSweep :type Boolean) (SweepResult :type Hit%20Result%20Structure%20%28by%20ref%29))
  (bind _sphere (Variables|Default|GetSphere))
  (if (== OtherActor (Variables|Default|GetAs%20BP%20First%20Person%20Character))
    (bind _asbp_first_person_character (Utilities|Casting|CastToBP_FirstPersonCharacter OtherActor))
    (Character|LaunchCharacter _asbp_first_person_character "0.000000,0.000000,3500.000000" false true)
    (Utilities|Time|SetTimerbyFunctionName 0 "Wait" 3.0 false false 3.0)
    (Rendering|SetVisibility _sphere false false)
    (Collision|SetCollisionEnabled _sphere "NoCollision")))

(event OnComponentBeginOverlap(Box)
  (params (OverlappedComponent :type Primitive%20Component%20Object%20Reference) (OtherActor :type Actor%20Object%20Reference) (OtherComp :type Primitive%20Component%20Object%20Reference) (OtherBodyIndex :type Integer) (bFromSweep :type Boolean) (SweepResult :type Hit%20Result%20Structure%20%28by%20ref%29))
  (if (== OtherActor (Variables|Default|GetAs%20BP%20First%20Person%20Character))
    (Utilities|FlowControl|DoOnce false
      (:Completed
        (Components|Activation|Activate (Variables|Default|GetInterpToMovement) false)))))

(event EventBeginPlay
  (bind _asbp_first_person_character (Utilities|Casting|CastToBP_FirstPersonCharacter (Game|GetPlayerCharacter 0)))
  (Variables|Default|SetAs%20BP%20First%20Person%20Character _asbp_first_person_character))

(event Collision|EventActorBeginOverlap
  (params (OtherActor :type Actor%20Object%20Reference)))

(event EventTick
  (params (DeltaSeconds :type Float%20%28single-precision%29)))

(fn ConstructionScript)