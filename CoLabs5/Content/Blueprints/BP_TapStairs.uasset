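; BP_TapStairs is a stairs hazard with a rotating tap handle that temporarily makes the first-person player slippery.
; Entering Box strips walking friction and braking, lowers the walkable floor angle, spins Handle and stretches StaticMesh2 vertically through a timeline.
; A three-second Delay on timeline updates restores movement and stops the handle, while a second, reversed timeline rescales the mesh afterwards.
; The player entering Box1 activates InterpToMovement once.
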(event OnComponentBeginOverlap(Box)
  (params (OverlappedComponent :type Primitive%20Component%20Object%20Reference) (OtherActor :type Actor%20Object%20Reference) (OtherComp :type Primitive%20Component%20Object%20Reference) (OtherBodyIndex :type Integer) (bFromSweep :type Boolean) (SweepResult :type Hit%20Result%20Structure%20%28by%20ref%29))
  (bind _asbp_first_person_character (Utilities|Casting|CastToBP_FirstPersonCharacter OtherActor))
  (Variables|/Script/Engine.CharacterMovementComponent|SetGroundFriction (Variables|/Script/Engine.Character|GetCharacterMovement _asbp_first_person_character) 0.0)
  (Variables|/Script/Engine.CharacterMovementComponent|SetBrakingDecelerationWalking (Variables|/Script/Engine.Character|GetCharacterMovement _asbp_first_person_character) 1.0)
  (Variables|/Script/Engine.CharacterMovementComponent|SetBrakingFrictionFactor (Variables|/Script/Engine.Character|GetCharacterMovement _asbp_first_person_character) 0.0)
  (Pawn|Components|CharacterMovement|SetWalkableFloorAngle (Variables|/Script/Engine.Character|GetCharacterMovement _asbp_first_person_character) 2e+01)
  (Variables|Default|SetHandleRotate true)
  (bind _newtrack_0 (Timeline|Timeline PlayFromStart)
    (:Update
      (Transformation|SetWorldScale3D (Variables|Default|GetStaticMesh2) (Math|Vector|MakeVector 1.3 1.3 (* _newtrack_0 3.0)))
      (Utilities|FlowControl|Delay 3.0)
      (bind _asbp_first_person_character_2 (Utilities|Casting|CastToBP_FirstPersonCharacter OtherActor))
      (Variables|/Script/Engine.CharacterMovementComponent|SetGroundFriction (Variables|/Script/Engine.Character|GetCharacterMovement _asbp_first_person_character_2) 8.0)
      (Variables|/Script/Engine.CharacterMovementComponent|SetBrakingDecelerationWalking (Variables|/Script/Engine.Character|GetCharacterMovement _asbp_first_person_character_2) 2e+03)
      (Variables|/Script/Engine.CharacterMovementComponent|SetBrakingFrictionFactor (Variables|/Script/Engine.Character|GetCharacterMovement _asbp_first_person_character_2) 1.0)
      (Pawn|Components|CharacterMovement|SetWalkableFloorAngle (Variables|/Script/Engine.Character|GetCharacterMovement _asbp_first_person_character_2) 45.0)
      (Variables|Default|SetHandleRotate false))
    (:Finished
      (bind _newtrack_0_2 (Timeline|Timeline_0 ReverseFromEnd)
        (:Update
          (Transformation|SetWorldScale3D (Variables|Default|GetStaticMesh2) (Math|Vector|MakeVector 1.3 1.3 (* _newtrack_0_2 4.0))))))))

(event OnComponentBeginOverlap(Box1)
  (params (OverlappedComponent :type Primitive%20Component%20Object%20Reference) (OtherActor :type Actor%20Object%20Reference) (OtherComp :type Primitive%20Component%20Object%20Reference) (OtherBodyIndex :type Integer) (bFromSweep :type Boolean) (SweepResult :type Hit%20Result%20Structure%20%28by%20ref%29))
  (if (== OtherActor (Variables|Default|GetAs%20BP%20First%20Person%20Character))
    (Utilities|FlowControl|DoOnce false
      (:Completed
        (Components|Activation|Activate (Variables|Default|GetInterpToMovement) false)))))

(event EventBeginPlay
  (bind _asbp_first_person_character (Utilities|Casting|CastToBP_FirstPersonCharacter (Game|GetPlayerCharacter 0)))
  (Variables|Default|SetAs%20BP%20First%20Person%20Character _asbp_first_person_character))

(event Collision|EventActorBeginOverlap
  (params (OtherActor :type Actor%20Object%20Reference)))

(event EventTick
  (params (DeltaSeconds :type Float%20%28single-precision%29))
  (if (Variables|Default|GetHandleRotate)
    (Transformation|AddLocalRotation (Variables|Default|GetHandle) "0.000000,0.000000,2.000000" false false)))

(fn ConstructionScript)